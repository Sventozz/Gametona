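; BP_ScaleBox is an interactable actor that toggles the scale of the Vendor that owns it.
; Interaction casts the owner to Vendor and flips its Scene component between normal and double world scale.
; The pure scale check re-evaluates after the change, so the debug print shows the next toggle value.
; Parent Interaction runs only when the scale has just returned to normal.
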(event EventBeginPlay
  (|CallParentFunction) ; This node is disabled and will not be called.\nDrag off pins to build functionality.
)

(event Collision|EventActorBeginOverlap
  (params (OtherActor :type Actor%20Object%20Reference))
  (|CallParentFunction OtherActor) ; This node is disabled and will not be called.\nDrag off pins to build functionality.
)

(event EventTick
  (params (DeltaSeconds :type Float%20%28single-precision%29))
  (|CallParentFunction DeltaSeconds) ; This node is disabled and will not be called.\nDrag off pins to build functionality.
)

(fn ConstructionScript
  (|CallParentFunction))

(fn Interaction
  (bind _asvendor (Utilities|Casting|CastToVendor (Components|GetOwner)))
  (Transformation|SetWorldScale3D (Variables|/Game/BaseActor.BaseActor_C|GetScene _asvendor) (select (Class|KismetMathLibrary|NotEqualExactlyVectorVector (.Scale (Math|Transform|BreakTransform (Transformation|GetWorldTransform (Variables|/Game/BaseActor.BaseActor_C|GetScene _asvendor)))) "1.000000,1.000000,1.000000") "1.000000,1.000000,1.000000" "2.000000,2.000000,2.000000"))
  (Development|PrintString (Utilities|String|ToString(Vector) (select (Class|KismetMathLibrary|NotEqualExactlyVectorVector (.Scale (Math|Transform|BreakTransform (Transformation|GetWorldTransform (Variables|/Game/BaseActor.BaseActor_C|GetScene _asvendor)))) "1.000000,1.000000,1.000000") "1.000000,1.000000,1.000000" "2.000000,2.000000,2.000000")))
  (if (not (Class|KismetMathLibrary|NotEqualExactlyVectorVector (.Scale (Math|Transform|BreakTransform (Transformation|GetWorldTransform (Variables|/Game/BaseActor.BaseActor_C|GetScene _asvendor)))) "1.000000,1.000000,1.000000"))
    (|CallParentFunction)))