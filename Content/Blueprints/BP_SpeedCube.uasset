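; BP_SpeedCube is an interactable pickup-style actor, named for speed, that triggers a timer on the player character.
; Its Interaction override finds every TopDownCharacter overlapping SphereColliderNew and calls StartTimer on each, then runs the parent Interaction.
; The timer's effect lives in the character, and the event graph holds only disabled default events.
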(event EventBeginPlay
  (|CallParentFunction) ; This node is disabled and will not be called.\nDrag off pins to build functionality.
)

(event Collision|EventActorBeginOverlap
  (params (OtherActor :type Actor%20Object%20Reference))
  (|CallParentFunction OtherActor) ; This node is disabled and will not be called.\nDrag off pins to build functionality.
)

(event EventTick
  (params (DeltaSeconds :type Float%20%28single-precision%29))
  (|CallParentFunction DeltaSeconds) ; This node is disabled and will not be called.\nDrag off pins to build functionality.
)

(fn ConstructionScript
  (|CallParentFunction))

(fn Interaction
  (for _array_element (Collision|GetOverlappingActors (Variables|Default|GetSphereColliderNew) "/Game/Blueprints/TopDownCharacter.TopDownCharacter_C" :!class /Script/Engine.PrimitiveComponent)
    (bind _astop_down_character (Utilities|Casting|CastToTopDownCharacter _array_element))
    (Class|GametonaCharacter|StartTimer _astop_down_character))
  (|CallParentFunction))