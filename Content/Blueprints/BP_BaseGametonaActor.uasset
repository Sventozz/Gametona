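; BP_BaseGametonaActor is a base interactable Gametona actor with a toggleable helper text label.
; Its construction script hides the TextRender component.
; ShowHelper calls its parent, flips the text's visibility through a FlipFlop, then removes the MenuUI widget held by BP_GametonaHUD from screen if valid.
; Interaction simply destroys the actor.
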(event EventShowHelper
  ;[1 1 1] Show Helper
  (|CallParentFunction)
  (bind _isa (Utilities|FlowControl|FlipFlop)
    (:A
      _)
    (:B
      _))
  (Rendering|SetVisibility (Variables|Default|GetTextRender) _isa false)
  (bind _asbp_gametona_hud (Utilities|Casting|CastToBP_GametonaHUD (HUD|GetHUD (Game|GetPlayerController 0))))
  (if (Utilities|IsValid (Variables|/Game/Core/BP_GametonaHUD.BP_GametonaHUD_C|GetMenuUI _asbp_gametona_hud))
    (Widget|RemovefromParent (Variables|/Game/Core/BP_GametonaHUD.BP_GametonaHUD_C|GetMenuUI _asbp_gametona_hud))))

(fn ConstructionScript
  (|CallParentFunction)
  (Rendering|SetVisibility (Variables|Default|GetTextRender) false false))

(fn Interaction
  (Actor|DestroyActor))