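; BP_Vendor is a shop actor that opens a buy menu and spawns purchasable cubes.
; Interaction shows the menu through BP_GametonaHUD and binds an event to its buy-item click.
; SpawnItems picks a speed, 3-press or scale cube class from the item's type, spawns it at the spawn marker with randomized world Y, then closes the menu.
; The menu also closes when the TopDownCharacter leaves the sphere collider.
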(event OnComponentEndOverlap(SphereColliderNew)
  (params (OverlappedComponent :type Primitive%20Component%20Object%20Reference) (OtherActor :type Actor%20Object%20Reference) (OtherComp :type Primitive%20Component%20Object%20Reference) (OtherBodyIndex :type Integer))
  (Utilities|Casting|CastToTopDownCharacter OtherActor)
  (CallFunction|CloseMenu))

(event EventBeginPlay
  (|CallParentFunction) ; This node is disabled and will not be called.\nDrag off pins to build functionality.
)

(event Collision|EventActorBeginOverlap
  (params (OtherActor :type Actor%20Object%20Reference))
  (|CallParentFunction OtherActor) ; This node is disabled and will not be called.\nDrag off pins to build functionality.
)

(event EventTick
  (params (DeltaSeconds :type Float%20%28single-precision%29))
  (|CallParentFunction DeltaSeconds) ; This node is disabled and will not be called.\nDrag off pins to build functionality.
)

(fn ConstructionScript
  (|CallParentFunction))

(fn Interaction
  (bind _asbp_gametona_hud (Utilities|Casting|CastToBP_GametonaHUD (HUD|GetHUD (Game|GetPlayerController 0)))
    (:then
      (Default|ShowUI _asbp_gametona_hud)
      (EventDispatchers|BindEventtoOnClickButtonBuyItem (Variables|/Game/Core/BP_GametonaHUD.BP_GametonaHUD_C|GetMenuUI _asbp_gametona_hud) (EventDispatchers|CreateEvent :!event SpawnItems)))
    (:CastFailed
      (Development|PrintString "Error: Cast to HUD - Failed"))))

(fn SpawnItems
  (params (ItemProperties :type Item%20Properties%20Structure))
  (bind _spawnlocationfor1item (Variables|Default|GetSpawnLocationFor1Item))
  (bind _returnvalue (Transformation|GetWorldTransform _spawnlocationfor1item))
  (bind (_location _rotation _scale) (Math|Transform|BreakTransform _returnvalue))
  (bind (_x _y _z) (Math|Vector|BreakVector _location))
  (Game|SpawnActorfromClass (Utilities|Select :Index (.CubeType (Utilities|Struct|BreakItemProperties ItemProperties)) :NewEnumerator0 "/Game/Blueprints/BP_SpeedCube.BP_SpeedCube_C" :NewEnumerator1 "/Game/Blueprints/BP_3PressCube.BP_3PressCube_C" :NewEnumerator2 "/Game/Blueprints/BP_ScaleBox.BP_ScaleBox_C") (Math|Transform|MakeTransform (Math|Vector|MakeVector _x (Math|Random|RandomFloatinRange -4e+02 4e+02) _z) _rotation _scale) "AlwaysSpawn" self 0)
  (CallFunction|CloseMenu))

(fn CloseMenu
  (bind _asbp_gametona_hud (Utilities|Casting|CastToBP_GametonaHUD (HUD|GetHUD (Game|GetPlayerController 0))))
  (if (Utilities|IsValid (Variables|/Game/Core/BP_GametonaHUD.BP_GametonaHUD_C|GetMenuUI _asbp_gametona_hud))
    (Widget|RemovefromParent (Variables|/Game/Core/BP_GametonaHUD.BP_GametonaHUD_C|GetMenuUI _asbp_gametona_hud))))