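; Vendor actor that opens a shop UI and can spawn purchasable cube items in the world.
; Interaction shows the menu through GametonaHUD and binds an event to its buy-item button, printing an error if the HUD cast fails.
; SpawnItems maps the item's cube type to a Speed, 3Press or Scale cube class.
; It spawns that cube at the spawn marker's transform, replacing Y with a random world coordinate.
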(event EventBeginPlay
  (|CallParentFunction) ; This node is disabled and will not be called.\nDrag off pins to build functionality.
)

(event Collision|EventActorBeginOverlap
  (params (OtherActor :type Actor%20Object%20Reference))
  (|CallParentFunction OtherActor) ; This node is disabled and will not be called.\nDrag off pins to build functionality.
)

(event EventTick
  (params (DeltaSeconds :type Float%20%28single-precision%29))
  (|CallParentFunction DeltaSeconds) ; This node is disabled and will not be called.\nDrag off pins to build functionality.
)

(fn ConstructionScript
  (|CallParentFunction))

(fn Interaction
  (bind _asgametona_hud (Utilities|Casting|CastToGametonaHUD (HUD|GetHUD (Game|GetPlayerController 0)))
    (:then
      (Default|ShowUI _asgametona_hud)
      (EventDispatchers|BindEventtoOnClickButtonBuyItem (Variables|/Game/GametonaHUD.GametonaHUD_C|GetMenuUI _asgametona_hud) (EventDispatchers|CreateEvent :!event SpawnItems)))
    (:CastFailed
      (Development|PrintString "Error: Cast to HUD - Failed"))))

(fn SpawnItems
  (params (ItemProperties :type Item%20Properties%20Structure))
  (bind _spawnlocationfor1item (Variables|Default|GetSpawnLocationFor1Item))
  (bind _returnvalue (Transformation|GetWorldTransform _spawnlocationfor1item))
  (bind (_location _rotation _scale) (Math|Transform|BreakTransform _returnvalue))
  (bind (_x _y _z) (Math|Vector|BreakVector _location))
  (Game|SpawnActorfromClass (Utilities|Select :Index (.CubeType (Utilities|Struct|BreakItemProperties ItemProperties)) :NewEnumerator0 "/Game/BP_SpeedCube.BP_SpeedCube_C" :NewEnumerator1 "/Game/BP_3PressCube.BP_3PressCube_C" :NewEnumerator2 "/Game/BP_ScaleBox.BP_ScaleBox_C") (Math|Transform|MakeTransform (Math|Vector|MakeVector _x (Math|Random|RandomFloatinRange -4e+02 4e+02) _z) _rotation _scale) "AlwaysSpawn" self 0))