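; Gametona HUD Blueprint that puts the coins and menu widgets on screen for player controller 0.
; BeginPlay creates the CoinsUI widget and adds it to the viewport.
; ShowUI removes any existing menu, then creates a fresh MenuUI widget and stores it, while HideUI removes the stored menu from the viewport.
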(event Custom|ShowUI
  (Development|PrintString "ShowUI")
  (Utilities|IsValid (Variables|Default|GetMenuUI)
    (:Is%20Valid
      (Widget|RemovefromParent (Variables|Default|GetMenuUI)))
    (:Is%20Not%20Valid
      _))
  (bind _returnvalue (UserInterface|CreateWidget "/Game/TopDownCPP/Widgets/MenuUI.MenuUI_C" (Game|GetPlayerController 0)))
  (UserInterface|Viewport|AddtoViewport _returnvalue 0)
  (Variables|Default|SetMenuUI _returnvalue))

(event EventBeginPlay
  (bind _returnvalue (UserInterface|CreateWidget "/Game/TopDownCPP/Widgets/CoinsUI.CoinsUI_C" (Game|GetPlayerController 0)))
  (UserInterface|Viewport|AddtoViewport _returnvalue 0))

(fn ConstructionScript)

(fn HideUI
  (bind _menuui (Variables|Default|GetMenuUI))
  (Utilities|IsValid _menuui
    (:Is%20Valid
      (Widget|RemovefromParent _menuui))))